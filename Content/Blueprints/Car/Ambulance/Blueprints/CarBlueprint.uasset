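; Player-driven ambulance vehicle pawn with steering, throttle, handbrake, camera yaw and right-click projectile firing from above the car.
; Tick writes velocity, scaled to approximate km/h, to a speedometer text.
; A Gate opened while the controlled pawn's up vector points down or sideways eases it upright, also pulling yaw toward zero.
; F or gamepad left face button instantly rights the mesh, keeping its yaw.
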(event `Key|RightMouseButton`
  (params (Key :type "Key Structure"))
  ;[1 1 1] Projectile Shooting Mechanism
  (:`Pressed`
    (`|SpawnActorFromClass` "/Game/Blueprints/Projectile/ProjectileBP.ProjectileBP_C" (`KismetMathLibrary.MakeTransform` (+ (.location (`self.GetTransform`)) (0.0 0.0 400.0)) (`KismetMathLibrary.MakeRotator` (.roll (`self.K2_GetActorRotation`)) (- (.pitch (`self.K2_GetActorRotation`)) 5.0) (.yaw (`self.K2_GetActorRotation`))) (.scale (`self.GetTransform`))) "Undefined" "OverrideRootScale" null null)))

(event `InputAxis|TurnLeft_Right`
  (params (AxisValue :type "Float (single-precision)"))
  ;[1 1 1] Steering
  (`WheeledVehicleMovementComponent.SetSteeringInput` (`self.VehicleMovement`) AxisValue))

(event `self.ReceiveBeginPlay`
  ;[1 1 1] Collision Detection And View (Connect ONLY when playtesting in vehicle blocking level)
)

(event `InputAction|Jump`
  (params (Key :type "Key Structure"))
  (bind _vehiclemovement (`self.VehicleMovement`))
  ;[1 1 1] Handbrake Control
  (:`Pressed`
    (`WheeledVehicleMovementComponent.SetHandbrakeInput` _vehiclemovement true))
  (:`Released`
    (`WheeledVehicleMovementComponent.SetHandbrakeInput` _vehiclemovement false)))

(event `InputAxis|MoveForward_Backward`
  (params (AxisValue :type "Float (single-precision)"))
  ;[1 1 1] Accelerate
  (`WheeledVehicleMovementComponent.SetThrottleInput` (`self.VehicleMovement`) AxisValue))

(event `InputAxis|Turn`
  (params (AxisValue :type "Float (single-precision)"))
  ;[1 1 1] Camera Control
  (`self.AddControllerYawInput` AxisValue))

(event `self.ReceiveTick`
  (params (DeltaSeconds :type "Float (single-precision)"))
  (bind _returnvalue (`Controller.K2_GetPawn` (`GameplayStatics.GetPlayerController` 0)))
  (bind (_returnvalue_location _returnvalue_rotation _returnvalue_scale) (`KismetMathLibrary.BreakTransform` (`self.GetTransform` _returnvalue)))
  ;[1 1 1] Speedometer
  (`TextRenderComponent.K2_SetText` (`self.Kmp/h Display`) (`KismetTextLibrary.Conv_DoubleToText` (`KismetMathLibrary.NormalizeToRange` (`KismetMathLibrary.VSize` (`self.GetVelocity`)) 0.0 30.0) "HalfToEven"))
  ;[1 1 1] Auto Flip Detection
  (`self.CheckVector`)
  (`/Engine/EditorBlueprintResources/StandardMacros.Gate` true :!label _label
    (:`Exit`
      (`self.K2_SetActorTransform` _returnvalue (`KismetMathLibrary.TInterpTo` (`KismetMathLibrary.MakeTransform` _returnvalue_location _returnvalue_rotation _returnvalue_scale) (`KismetMathLibrary.MakeTransform` _returnvalue_location (`KismetMathLibrary.MakeRotator` 0.0 (.pitch _returnvalue_rotation)) _returnvalue_scale) DeltaSeconds 1.0) false true))))

(event `CheckVector`
  ;[1 1 1] Auto Flip Detection
  (if (<= (.z (`self.GetActorUpVector` (`Controller.K2_GetPawn` (`GameplayStatics.GetPlayerController` 0)))) 0.0)
    (goto _label :!via `Open`)
    (else
      (goto _label :!via `Close`))))

(event `Key|F`
  (params (Key :type "Key Structure"))
  (bind _mesh (`self.Mesh`))
  (bind (_returnvalue_location _returnvalue_rotation _returnvalue_scale) (`KismetMathLibrary.BreakTransform` (`SceneComponent.K2_GetComponentToWorld` _mesh)))
  ;[1 1 1] Manual Flip Detection
  (:`Pressed`
    (`SceneComponent.K2_SetWorldTransform` _mesh (`KismetMathLibrary.MakeTransform` _returnvalue_location (`KismetMathLibrary.MakeRotator` 0.0 0.0 (.yaw _returnvalue_rotation)) _returnvalue_scale) false true)))

(event `Key|Gamepad_FaceButton_Left`
  (params (Key :type "Key Structure"))
  (bind _mesh (`self.Mesh`))
  (bind (_returnvalue_location _returnvalue_rotation _returnvalue_scale) (`KismetMathLibrary.BreakTransform` (`SceneComponent.K2_GetComponentToWorld` _mesh)))
  ;[1 1 1] Manual Flip Detection
  (:`Pressed`
    (`SceneComponent.K2_SetWorldTransform` _mesh (`KismetMathLibrary.MakeTransform` _returnvalue_location (`KismetMathLibrary.MakeRotator` 0.0 0.0 (.yaw _returnvalue_rotation)) _returnvalue_scale) false true)))

(fn `UserConstructionScript`)